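; Base character Blueprint for RealityRoom that provides player movement and a simple recording state.
; InputGraph maps look and turn axes to controller pitch and yaw, move axes to actor-relative movement input, and the Jump action to Jump.
; Forward movement uses a local direction with both X and Z components.
; StartRecording sets a flag and stores the game-time start, and StopRecording clears the flag, with no capture logic here.
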(event EventBeginPlay)

(event Collision|EventActorBeginOverlap
  (params (OtherActor :type Actor%20Object%20Reference)))

(event EventTick
  (params (DeltaSeconds :type Float%20%28single-precision%29)))

(event EventBeginPlay)

(event Input|ActionEvents|InputActionJump
  (params (Key :type Key%20Structure))
  (:Pressed
    (Character|Jump)))

(event Input|AxisEvents|InputAxisLookUp
  (params (AxisValue :type Float%20%28single-precision%29))
  (Pawn|Input|AddControllerPitchInput AxisValue))

(event Input|AxisEvents|InputAxisTurn
  (params (AxisValue :type Float%20%28single-precision%29))
  (Pawn|Input|AddControllerYawInput AxisValue))

(event Input|AxisEvents|InputAxisMoveRight
  (params (AxisValue :type Float%20%28single-precision%29))
  (Pawn|Input|AddMovementInput (Math|Transform|TransformDirection (Transformation|GetActorTransform) "0.000000,1.000000,0.000000") AxisValue false))

(event Input|AxisEvents|InputAxisMoveForward
  (params (AxisValue :type Float%20%28single-precision%29))
  (Pawn|Input|AddMovementInput (Math|Transform|TransformDirection (Transformation|GetActorTransform) "1.000000,0.000000,1.000000") AxisValue false))

(fn ConstructionScript)

(fn StartRecording
  (Variables|Default|SetIsRecording true)
  (Variables|Default|SetRecordStartTime (Utilities|Time|GetGameTimeinSeconds)))

(fn StopRecording
  (Variables|Default|SetIsRecording false))