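; FakePlayerController_BP is a player controller that records player input while IsRecording is set, despite its "fake" name.
; Each tick, after the parent tick, it appends a RealityRoomInput entry to InputBuffer.
; Each entry holds the movement, look and turn axes, the controlled Character's jump press, and a game-time timestamp shifted back by one second.
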(event EventTick
  (params (DeltaSeconds :type Float%20%28single-precision%29))
  (|CallParentFunction DeltaSeconds)
  (if (Variables|Default|GetIsRecording)
    (Utilities|Array|Add (Variables|Default|GetInputBuffer) (Utilities|Struct|MakeRealityRoomInput (Input|AxisValues|GetMoveForward) (Input|AxisValues|GetMoveRight) (Input|AxisValues|GetLookUp) (Input|AxisValues|GetTurn) (Variables|/Script/Engine.Character|GetbPressedJump (.AsCharacter (Utilities|Casting|CastToCharacter (Pawn|GetControlledPawn)))) false (- (Utilities|Time|GetGameTimeinSeconds) 1.0)))))

(fn ConstructionScript)