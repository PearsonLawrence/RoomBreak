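; Actor that toggles in-game visibility across its AffectedActors array, showing selected indices and hiding others, or the inverse when ShouldHideInstead is set.
; BeginPlay passes InitialIndices to Reveal, which applies the state to those targets and collects the remaining indices in RejectedList.
; Reveal never clears RejectedList and indexes it by its own values when applying the opposite state.
; RevealByIndex switches exclusively to one entry, inverting all others.
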(event EventBeginPlay
  (CallFunction|Reveal (Variables|Selector|GetInitialIndices)))

(fn ConstructionScript)

(fn RevealbyIndex
  (params (Index :type Integer))
  (bind _hidden (CallFunction|GetNewHiddenValue))
  (bind _returnvalue (not _hidden))
  (Rendering|SetActorHiddenInGame (Utilities|Array|Get(acopy) (Variables|Selector|GetAffectedActors) Index) (CallFunction|GetNewHiddenValue))
  (Utilities|FlowControl|Sequence
    (:then_0
      (for _index (range 0 (- Index 1))
        (Rendering|SetActorHiddenInGame (Utilities|Array|Get(acopy) (Variables|Selector|GetAffectedActors) _index) _returnvalue)))
    (:then_1
      (for _index_2 (range (+ Index 1) (- (Utilities|Array|Length (Variables|Selector|GetAffectedActors)) 1))
        (Rendering|SetActorHiddenInGame (Utilities|Array|Get(acopy) (Variables|Selector|GetAffectedActors) _index_2) _returnvalue)))))

(fn Reveal
  (params (Targets :type Array%20of%20Integers))
  (bind _affectedactors (Variables|Selector|GetAffectedActors))
  (bind _rejectedlist (LocalVariables|GetRejectedList))
  (Utilities|FlowControl|Sequence
    (:then_0
      (if (not (> (Utilities|Array|Length (Variables|Selector|GetAffectedActors)) 0))
        (return)))
    (:then_1
      (for _index (range 0 (- (Utilities|Array|Length (Variables|Selector|GetAffectedActors)) 1))
        (if (== (Utilities|Array|FindItem Targets _index) -1)
          (Utilities|Array|Add (LocalVariables|GetRejectedList) _index))))
    (:then_2
      (for _array_element Targets
        (Rendering|SetActorHiddenInGame (Utilities|Array|Get(acopy) _affectedactors _array_element) (CallFunction|GetNewHiddenValue))))
    (:then_3
      (for _array_element_2 _rejectedlist
        (Rendering|SetActorHiddenInGame (Utilities|Array|Get(acopy) _affectedactors (Utilities|Array|Get(acopy) _rejectedlist _array_element_2)) (not (CallFunction|GetNewHiddenValue)))))))

(fn GetNewHiddenValue
  (return (Variables|Selector|GetShouldHideInstead)))