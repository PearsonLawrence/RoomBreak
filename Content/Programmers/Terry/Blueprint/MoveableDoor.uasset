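; MoveableDoor is a lockable door actor that swings open around its vertical axis when interacted with or told to open.
; Interact and OpenDoor set an opening flag if unlocked, and Tick rotates the door at constant speed toward its open angle over a configurable time.
; A RoomBreakCharacter overlapping the Cube while opening triggers Reset on its Resetvalue and on the door.
; ResetDoor restores the closed state, while OnLock and OnUnlock toggle the lock.
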(event OnComponentBeginOverlap(Cube)
  (params (OverlappedComponent :type Primitive%20Component%20Object%20Reference) (OtherActor :type Actor%20Object%20Reference) (OtherComp :type Primitive%20Component%20Object%20Reference) (OtherBodyIndex :type Integer) (bFromSweep :type Boolean) (SweepResult :type Hit%20Result%20Structure%20%28by%20ref%29))
  (if (Variables|Default|GetIsOpening)
    (bind _asroom_break_character (Utilities|Casting|CastToRoomBreakCharacter OtherActor))
    (Default|Reset (Variables|/Game/Programmers/Pearson/Blueprint/Player/RoomBreakCharacter.RoomBreakCharacter_C|GetResetvalue _asroom_break_character))
    (CallFunction|Reset)))

(event Custom|OpenDoor
  (if (not (Variables|Default|GetLocked))
    (Variables|Default|SetIsOpening true)
    (Variables|Default|SetLastInteractionTime (Utilities|Time|GetGameTimeinSeconds))))

(event Custom|ResetDoor
  (Transformation|SetRelativeRotation (Variables|Default|GetDoor) "0, 0, 0" false false)
  (Variables|Default|SetLastInteractionTime 0.0)
  (Variables|Default|SetIsOpening false))

(event Custom|OnUnlock
  (Variables|Default|SetLocked false))

(event Custom|OnLock
  (Variables|Default|SetLocked true))

(event EventBeginPlay)

(event EventReset)

(event EventUnlock)

(event EventLock)

(event EventTick
  (params (DeltaSeconds :type Float%20%28single-precision%29))
  (if (Variables|Default|GetIsOpening)
    (Transformation|SetRelativeRotation (Variables|Default|GetDoor) (Class|KismetMathLibrary|RInterptoConstant (Variables|/Script/Engine.SceneComponent|GetRelativeRotation (Variables|Default|GetDoor)) (Math|Conversions|RotationFromXVector (Math|Vector|RotateVectorAroundAxis "1.000000, 0, 0" (Variables|Default|GetOpenDoorAngle) "0, 0,1.000000")) DeltaSeconds (/ (Variables|Default|GetOpenDoorAngle) (Variables|Default|GetTimeToOpen))) false false)))

(event EventInteract
  (params (Caller :type Actor%20Object%20Reference))
  (if (not (Variables|Default|GetLocked))
    (Variables|Default|SetIsOpening true)
    (Variables|Default|SetLastInteractionTime (Utilities|Time|GetGameTimeinSeconds))))

(fn ConstructionScript)