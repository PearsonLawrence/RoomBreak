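; First-person player character that interacts with knife pickups and doors and records a trail of its movement.
; Each tick, a forward camera sphere trace sets the interactable; E grabs a knife or, on a TempDoor, calls Reset on Resetvalue.
; A 0.2-second Delay throttles logging of debug-drawn, flattened positions and idle times into WaypointManager's CookieArray.
; Its Reset event teleports the player to StartLocation and restores control rotation.
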(event EventTick
  (params (DeltaSeconds :type Float%20%28single-precision%29))
  (bind _returnvalue (Transformation|GetActorLocation))
  (bind _waypointmanager (Variables|Default|GetWaypointManager))
  (bind _charactermovement (Variables|Character|GetCharacterMovement))
  (bind _returnvalue_2 (Transformation|GetActorLocation _waypointmanager))
  (bind _returnvalue_3 (Math|Vector|MakeVector (.x _returnvalue) (.y _returnvalue) 0.0))
  (bind _velocity (Variables|/Script/Engine.MovementComponent|GetVelocity _charactermovement))
  (bind _returnvalue_4 (+ _returnvalue_3 _returnvalue_2))
  (CallFunction|TraceforInteractable)
  (Utilities|FlowControl|Delay 0.2)
  (Rendering|Debug|DrawDebugSphere _returnvalue_4 2e+01 12 "(R=0.000000,G=0.000000,B=0.000000,A=1.000000)" 1e+01 1.0)
  (if (and (<= (.x _velocity) 0.0) (<= (.y _velocity) 0.0))
    (Variables|Default|SetStoreTime 0.2)
    (else
      (Variables|Default|SetStoreTime 0.0)))
  (Utilities|Array|Add (Variables|/Game/Programmers/Pearson/Blueprint/AI/WaypointManager.WaypointManager_C|GetCookieArray _waypointmanager) (Utilities|Struct|MakeWaypointInformation _returnvalue_4 (Variables|Default|GetStoreTime))))

(event EventReset
  (bind _startlocation (Variables|Default|GetStartLocation))
  (Transformation|SetActorLocation (.location _startlocation) false true)
  (Pawn|SetControlRotation (Pawn|GetController) (.rotation _startlocation)))

(event Input|KeyboardEvents|E
  (params (Key :type Key%20Structure))
  (bind _interactableobject (Variables|Default|GetInteractableObject))
  (:Pressed
    (bind _asknife_pickup_bp (Utilities|Casting|CastToKnifePickupBP _interactableobject)
      (:then
        (Actor|DestroyActor _asknife_pickup_bp)
        (Variables|Default|SetGrabbedKnife true)
        (Rendering|SetVisibility (Variables|Default|GetStaticMesh) true false))
      (:CastFailed
        (Utilities|Casting|CastToTempDoor _interactableobject)
        (Default|Reset (Variables|Default|GetResetvalue))))))

(fn ConstructionScript)

(fn TraceforInteractable
  (bind _firstpersoncameracomponent (Variables|Default|GetFirstPersonCameraComponent))
  (bind _returnvalue (Transformation|GetWorldLocation _firstpersoncameracomponent))
  (bind (_outhit _returnvalue_2) (Collision|SphereTraceByChannel _returnvalue (+ _returnvalue (* (Math|Vector|GetForwardVector _firstpersoncameracomponent) 1e+02)) 2e+01 "TraceTypeQuery3" false 0 "ForOneFrame"))
  (bind _output_get (Variables|Default|SetCanInteract _returnvalue_2))
  (if _output_get
    (Variables|Default|SetInteractableObject (.hitactor _outhit))
    (else
      (Variables|Default|SetInteractableObject 0))))