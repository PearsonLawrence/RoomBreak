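; TempReset is a reset manager that spawns PlayerSelfAI copies of the player's past runs across eight point-marked start locations.
; On BeginPlay it caches those transforms and registers itself with the RoomBreakCharacter.
; Each Reset spawns an AI at the current point and hands it the player's recorded waypoints, then clears the recording.
; It then advances the player's start, resets the player and revives accumulated AIs, teleporting earlier ones back to their points.
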(event EventBeginPlay
  (bind _locations (Variables|Default|GetLocations))
  (bind _outactors (Actor|GetAllActorsOfClass "/Game/Programmers/Pearson/Blueprint/Player/RoomBreakCharacter.RoomBreakCharacter_C"))
  (bind _output_get (Variables|Default|SetPlayer (Utilities|Array|Get(acopy) _outactors)))
  (Variables|/Game/Programmers/Pearson/Blueprint/Player/RoomBreakCharacter.RoomBreakCharacter_C|SetResetvalue _output_get self)
  (Utilities|Array|Add _locations (Transformation|GetWorldTransform (Variables|Default|GetPoint0)))
  (Utilities|Array|Add _locations (Transformation|GetWorldTransform (Variables|Default|GetPoint1)))
  (Utilities|Array|Add _locations (Transformation|GetWorldTransform (Variables|Default|GetPoint2)))
  (Utilities|Array|Add _locations (Transformation|GetWorldTransform (Variables|Default|GetPoint3)))
  (Utilities|Array|Add _locations (Transformation|GetWorldTransform (Variables|Default|GetPoint4)))
  (Utilities|Array|Add _locations (Transformation|GetWorldTransform (Variables|Default|GetPoint5)))
  (Utilities|Array|Add _locations (Transformation|GetWorldTransform (Variables|Default|GetPoint6)))
  (Utilities|Array|Add _locations (Transformation|GetWorldTransform (Variables|Default|GetPoint7))))

(event Collision|EventActorBeginOverlap
  (params (OtherActor :type Actor%20Object%20Reference)))

(event EventTick
  (params (DeltaSeconds :type Float%20%28single-precision%29)))

(event EventReset
  (bind _currentai (Variables|Default|GetCurrentAI))
  (bind _locations (Variables|Default|GetLocations))
  (bind _currentreset (Variables|Default|GetCurrentReset))
  (bind _currentai_2 (Variables|Default|GetCurrentAI))
  (bind _player (Variables|Default|GetPlayer))
  (bind _output (Utilities|Array|Get(acopy) _locations _currentreset))
  (bind _waypointmanager (Variables|/Game/Programmers/Pearson/Blueprint/Player/RoomBreakCharacter.RoomBreakCharacter_C|GetWaypointManager _player))
  (bind (_location _rotation) (Math|Transform|BreakTransform _output))
  (bind _cookiearray (Variables|/Game/Programmers/Pearson/Blueprint/AI/WaypointManager.WaypointManager_C|GetCookieArray _waypointmanager))
  (bind _returnvalue (AI|SpawnAIFromClass "/Game/Programmers/Pearson/Blueprint/AI/PlayerSelfAI.PlayerSelfAI_C" 0 _location _rotation true))
  (bind _asplayer_self_ai (Utilities|Casting|CastToPlayerSelfAI _returnvalue))
  (if (<= (Utilities|Array|Length _currentai_2) 0)
    (Variables|/Game/Programmers/Pearson/Blueprint/AI/PlayerSelfAI.PlayerSelfAI_C|Settest _asplayer_self_ai true))
  (Utilities|Array|Add _currentai_2 _asplayer_self_ai)
  (Variables|/Game/Programmers/Pearson/Blueprint/AI/PlayerSelfAI.PlayerSelfAI_C|SetWaypoints _asplayer_self_ai _cookiearray)
  (Utilities|Array|Clear _cookiearray)
  (CallFunction|SetPlayerStartValueandIncramentArray _output)
  (for (_ _array_index) _currentai
    (Variables|/Game/Programmers/Pearson/Blueprint/AI/PlayerSelfAI.PlayerSelfAI_C|SetCurrentWaypoint (Utilities|Array|Get(acopy) _currentai _array_index) 0)
    (Variables|/Game/Programmers/Pearson/Blueprint/AI/PlayerSelfAI.PlayerSelfAI_C|SetIsDead (Utilities|Array|Get(acopy) _currentai _array_index) false)
    (Physics|SetSimulatePhysics (Variables|/Script/Engine.Character|GetMesh (Utilities|Array|Get(acopy) _currentai _array_index)) false)
    (Components|Activation|Activate (Variables|/Script/Engine.Character|GetCapsuleComponent (Utilities|Array|Get(acopy) _currentai _array_index)) false)
    (Components|Activation|Activate (Variables|/Script/Engine.Character|GetCharacterMovement (Utilities|Array|Get(acopy) _currentai _array_index)) false)
    (Collision|SetCollisionEnabled (Variables|/Script/Engine.Character|GetCapsuleComponent (Utilities|Array|Get(acopy) _currentai _array_index)) "QueryAndPhysics")
    (if (!= (Utilities|Array|Get(acopy) (Variables|Default|GetCurrentAI) (- _array_index 1)) 0)
      (Transformation|SetActorLocation (Utilities|Array|Get(acopy) (Variables|Default|GetCurrentAI) (- _array_index 1)) (.location (Utilities|Array|Get(acopy) (Variables|Default|GetLocations) (- _array_index 1))) false true)
      (Transformation|SetActorRotation (Utilities|Array|Get(acopy) (Variables|Default|GetCurrentAI) (- _array_index 1)) (.rotation (Utilities|Array|Get(acopy) (Variables|Default|GetLocations) (- _array_index 1))) true))))

(fn ConstructionScript)

(fn SetPlayerStartValueandIncramentArray
  (params (StartLocation :type Transform))
  (bind _player (Variables|Default|GetPlayer))
  (bind _result (Math|Integer|IncrementInt (Variables|Default|GetCurrentReset))
    (:%20%20
      (Variables|/Game/Programmers/Pearson/Blueprint/Player/RoomBreakCharacter.RoomBreakCharacter_C|SetStartLocation _player (Utilities|Array|Get(acopy) (Variables|Default|GetLocations) _result))
      (Default|Reset _player)
      (return _player))))