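; FinalAI is an interactable AI actor that shatters when used and flags the player character's Over state.
; On BeginPlay it caches the first RoomBreakCharacter in the level as Player.
; Interact spawns a DeathMan at its transform and damages that actor's Destructible to break it apart.
; It then sets Player.Over and hides its own mesh, so the destructible stands in for it.
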(event EventInteract
  (params (Caller :type Actor%20Object%20Reference))
  (bind _returnvalue (Transformation|GetActorLocation))
  (bind _returnvalue_2 (Game|SpawnActorfromClass "/Game/Blueprints/DeathMan.DeathMan_C" (Transformation|GetActorTransform) "AlwaysSpawn" 0 0))
  (Class|DestructibleComponent|ApplyDamage (Variables|/Game/Blueprints/DeathMan.DeathMan_C|GetDestructible _returnvalue_2) 1e+02 _returnvalue _returnvalue 5e+01)
  (Variables|/Game/Programmers/Pearson/Blueprint/Player/RoomBreakCharacter.RoomBreakCharacter_C|SetOver (Variables|Default|GetPlayer) true)
  (Rendering|SetVisibility (Variables|Character|GetMesh) false true))

(event EventBeginPlay
  (bind _outactors (Actor|GetAllActorsOfClass "/Game/Programmers/Pearson/Blueprint/Player/RoomBreakCharacter.RoomBreakCharacter_C"))
  (Variables|Default|SetPlayer (Utilities|Array|Get(acopy) _outactors)))

(fn ConstructionScript)