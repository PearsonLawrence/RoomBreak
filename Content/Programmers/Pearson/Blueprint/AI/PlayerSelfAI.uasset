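; AI character pawn, PlayerSelfAI, that registers itself with its Dude_Controller on BeginPlay and handles its own death.
; Die spawns a DeathMan at its transform, shatters it through destructible damage, flags itself dead and calls DeactivateAI.
; DeactivateAI switches off movement and capsule collision and hides the mesh.
; Waypoint movement, stab attack, death animation and ragdoll logic are left unconnected, and Tick does nothing.
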(event Custom|Deactivate%20AI
  (bind _capsulecomponent (Variables|Collision|GetCapsuleComponent))
  (Components|Activation|Deactivate (Variables|Character|GetCharacterMovement))
  (Components|Activation|Deactivate _capsulecomponent)
  (Collision|SetCollisionEnabled _capsulecomponent "NoCollision")
  (Rendering|SetVisibility (Variables|Character|GetMesh) false true))

(event Custom|Die
  (bind _returnvalue (Transformation|GetActorLocation))
  (bind _returnvalue_2 (Game|SpawnActorfromClass "/Game/Blueprints/DeathMan.DeathMan_C" (Transformation|GetActorTransform) "AlwaysSpawn" 0 0))
  (Class|DestructibleComponent|ApplyDamage (Variables|/Game/Blueprints/DeathMan.DeathMan_C|GetDestructible _returnvalue_2) 1e+02 _returnvalue _returnvalue 5e+01)
  (Variables|Default|SetIsDead true)
  (CallFunction|DeactivateAI))

(event EventTick
  (params (DeltaSeconds :type Float%20%28single-precision%29))
  (if (Variables|Default|Gettest)
    _))

(event EventBeginPlay
  (bind _asdude_controller (Utilities|Casting|CastToDude_Controller (Pawn|GetController)))
  (Variables|/Game/Programmers/Henry/AI/Dude_Controller.Dude_Controller_C|SetpawnRef _asdude_controller self)
  (Development|PrintString (Utilities|String|ToString(Integer) (Variables|Default|GetkillWaypointIndex)) true true "(R=1.000000,G=0.050213,B=0.000000,A=1.000000)"))

(fn ConstructionScript)